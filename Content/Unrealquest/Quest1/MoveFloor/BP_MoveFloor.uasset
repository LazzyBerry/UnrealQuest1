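; BP_MoveFloor is a moving floor that slides its static mesh between FirstPoint and EndPoint.
; While Moving is set, Tick plays or reverses the MovingCurve timeline according to IsReverse.
; The timeline lerps the mesh's relative location and flips IsReverse on finishing to swap direction.
; The construction script derives the timeline play rate from MovingTime.
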(event `self.ReceiveBeginPlay`)

(event `self.ReceiveTick`
  (params (DeltaSeconds :type "Float (single-precision)"))
  (if (`self.bMoving`)
    (if (`self.isReverse`)
      ;[1 1 1] 位置の更新
      (bind (_direction _timeline) (`Timeline|MovingCurve` :!label _label)
        (:`Update`
          (`SceneComponent.K2_SetRelativeLocation` (`self.StaticMesh`) (`KismetMathLibrary.VLerp` (`SceneComponent.RelativeLocation` (`self.FirstPoint`)) (`SceneComponent.RelativeLocation` (`self.EndPoint`)) _timeline) false false))
        (:`Finished`
          ;[1 1 1] 最後まで行ったら逆移動にする
          (set `self.isReverse` (not (`self.isReverse`)))))
      (else
        (goto _label :!via `Reverse`)))))

(fn `UserConstructionScript`
  ;[1 1 1] 移動速度を設定
  (`TimelineComponent.SetPlayRate` (`self.MovingCurve`) (/ 1.0 (`self.MovingTime`))))